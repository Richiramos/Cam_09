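; Construction-script tool that lays out grids of static meshes, likely boxes given the "cajas" name.
; Per-mesh count and spacing arrays are resized to match Listmesh, then each entry spawns individual StaticMeshComponents in X/Y rows using integer division and modulo.
; The Transform array meant to offset each grid is emptied before being read.
; The inner loop's end index equals X×Y, giving one component beyond each grid.
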(fn `UserConstructionScript`
  (bind _num (`self.Num`))
  (bind _returnvalue (`KismetArrayLibrary.Array_Length` (`self.Listmesh`)))
  (`KismetArrayLibrary.Array_Resize` _num _returnvalue)
  (`KismetArrayLibrary.Array_Resize` (`self.Space_X`) _returnvalue)
  (`KismetArrayLibrary.Array_Resize` (`self.Space_Y`) _returnvalue)
  (`KismetArrayLibrary.Array_Resize` (`self.Number_X`) _returnvalue)
  (`KismetArrayLibrary.Array_Resize` (`self.Number_Y`) _returnvalue)
  (`KismetArrayLibrary.Array_Resize` (`self.Transform`))
  (for (_ _array_index) _num
    (bind _output (`|GetArrayItem` (`self.Number_Y`) _array_index))
    (for _index (range (+ (- (* (`|GetArrayItem` (`self.Number_X`) _array_index) _output) 0) 1))
      (bind (_output_location _output_rotation _output_scale) (`KismetMathLibrary.BreakTransform` (`|GetArrayItem` (`self.Transform`) _array_index)))
      (bind _returnvalue_2 (`AddComponent|NODE_AddStaticMeshComponent-0` :`RelativeTransform` (`KismetMathLibrary.MakeTransform` (+ _output_location (`KismetMathLibrary.MakeVector` (* (/ _index _output) (`|GetArrayItem` (`self.Space_X`) _array_index)) (* (mod _index _output) (`|GetArrayItem` (`self.Space_Y`) _array_index)))) _output_rotation _output_scale)))
      (`StaticMeshComponent.SetStaticMesh` _returnvalue_2 (`|GetArrayItem` (`self.Listmesh`) _array_index)))))